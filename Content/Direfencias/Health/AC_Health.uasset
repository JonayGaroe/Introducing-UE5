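; AC_Health is a health component that tracks current health, maximum health and a death flag for its owner.
; INIT receives the maximum health and starts current health at that value.
; TakeDamage subtracts damage, clamps the result between zero and the maximum, then calls OnDead.
; OnDead only sets IsDead according to whether health has reached zero, with no further death handling or notification.
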(event `INIT`
  (params (MaxHealth :type "Float (double-precision)"))
  (bind _output_get (set `self.MaxHealth` MaxHealth))
  (set `self.CurHealth` _output_get))

(event `TakeDamage`
  (params (Damage :type "Float (double-precision)"))
  (set `self.CurHealth` (`KismetMathLibrary.FClamp` (- (`self.CurHealth`) Damage) 0.0 (`self.MaxHealth`)))
  (`self.OnDead`))

(event `OnDead`
  (if (<= (`self.CurHealth`) 0.0)
    (set `self.IsDead?` true)
    (else
      (set `self.IsDead?` false))))